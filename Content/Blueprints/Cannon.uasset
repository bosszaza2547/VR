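; Cannon actor that runs a single automatic firing sequence when play begins.
; A first timeline rotates the lever pivot from its starting rotation to an end rotation, then a second timeline does the same for the cannon pivot.
; When the second finishes, it spawns an enlarged Projectile at the Arrow component's location and rotation.
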(event EventBeginPlay
  (bind _arrow (Variables|Default|GetArrow))
  (bind _returnvalue (Transformation|GetWorldTransform _arrow))
  (Variables|Default|SetLever%20First%20Rotation (Variables|/Script/Engine.SceneComponent|GetRelativeRotation (Variables|Default|GetLever%20Rotation%20point)))
  (Variables|Default|SetCannon%20First%20Rotation (Variables|/Script/Engine.SceneComponent|GetRelativeRotation (Variables|Default|GetCannon%20Rotate%20Point)))
  (bind _time (Timeline|Timeline PlayFromStart)
    (:Update
      (Transformation|SetRelativeRotation (Variables|Default|GetLever%20Rotation%20point) (Math|Rotator|Lerp(Rotator) (Variables|Default|GetLever%20First%20Rotation) (Variables|Default|GetLever%20End%20Rotation) _time) false false))
    (:Finished
      (bind _time_2 (Timeline|Timeline_0 PlayFromStart)
        (:Update
          (Transformation|SetRelativeRotation (Variables|Default|GetCannon%20Rotate%20Point) (Math|Rotator|Lerp(Rotator) (Variables|Default|GetCannon%20First%20Rotation) (Variables|Default|GetCannon%20End%20Rotation) _time_2) false false))
        (:Finished
          (Game|SpawnActorfromClass "/Game/VRTemplate/Blueprints/Projectile.Projectile_C" (Math|Transform|MakeTransform (.location _returnvalue) (.rotation _returnvalue) "5.000000,5.000000,5.000000") "Undefined" "MultiplyWithRoot" 0 0))))))

(fn ConstructionScript)